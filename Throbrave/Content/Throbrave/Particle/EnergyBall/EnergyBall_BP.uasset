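; Energy ball actor that charges on spawn, then flies along negative world X once told to move.
; After the MoveDuration delay it flags its energy as full, exposed through a getter for other Blueprints to read.
; While IsMove is set externally, Tick shifts only the Niagara component by a fixed, frame-rate-dependent step without sweep.
; The actor destroys itself when that component's X drops below DestroyDistance.
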(event EventBeginPlay
  (Utilities|FlowControl|Delay (Variables|Default|GetMove%20Duration))
  (Variables|Default|SetIs%20EnergyFull true))

(event Collision|EventActorBeginOverlap
  (params (OtherActor :type Actor%20Object%20Reference)))

(event EventTick
  (params (DeltaSeconds :type Float%20%28single-precision%29))
  (bind _niagara (Variables|Default|GetNiagara))
  (bind _returnvalue (Transformation|GetWorldLocation _niagara))
  (if (Variables|Default|GetIsMove)
    (if (< (.x (Transformation|GetWorldLocation (Variables|Default|GetNiagara))) (Variables|Default|GetDestroy%20Distance))
      (Actor|DestroyActor)
      (else
        (Transformation|SetWorldLocation _niagara (Math|Vector|MakeVector (- (.x _returnvalue) 2e+01) (.y _returnvalue) (.z _returnvalue)) false false)))))

(fn ConstructionScript)

(fn GetIsMove
  (return (Variables|Default|GetIsMove)))

(fn SetIsMove
  (params (flag :type Boolean))
  (Variables|Default|SetIsMove flag))

(fn GetIsEnergyFull
  (return (Variables|Default|GetIs%20EnergyFull)))