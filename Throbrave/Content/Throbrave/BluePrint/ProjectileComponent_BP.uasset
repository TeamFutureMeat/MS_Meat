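; ProjectileComponent_BP is a component that makes a projectile home in on a target actor and detects when it arrives.
; An initialize function stores the movement component, target and parent actor, then sets the homing target to the target's box component matching a given tag, with the last match winning.
; Each tick it measures parent-to-target distance and sets a HitTarget flag once that falls below a minimum.
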(event EventBeginPlay)

(event EventTick
  (params (DeltaSeconds :type Float%20%28single-precision%29))
  (bind _output_get (Variables|Default|SetTargetDistance (Math|Vector|VectorLength (- (Transformation|GetActorLocation (Variables|Default|GetTarget)) (Transformation|GetActorLocation (Variables|Default|GetParentActor))))))
  (if (< _output_get (Variables|Default|GetMinTargetDistance))
    (Variables|Default|SetHitTarget true)))

(fn ProjectileComponentInitialize
  (params (ProjectileMovement :type Projectile%20Movement%20Component%20Object%20Reference) (TargetActor :type Actor%20Object%20Reference) (TargetTagName :type Name) (ParentActor :type Actor%20Object%20Reference))
  (bind _output_get (Variables|Default|SetProjectileMovement ProjectileMovement))
  (bind _output_get_2 (Variables|Default|SetTarget TargetActor))
  (Variables|Default|SetParentActor ParentActor)
  (for _array_element (Actor|GetComponentsbyTag _output_get_2 "/Script/Engine.BoxComponent" TargetTagName)
    (Variables|/Script/Engine.ProjectileMovementComponent|SetHomingTargetComponent _output_get _array_element)))