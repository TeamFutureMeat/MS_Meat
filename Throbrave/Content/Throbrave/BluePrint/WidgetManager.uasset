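; Manager actor that keeps Mission and Cutin widgets off screen while higher-priority UI or boss sequences are showing.
; Every Tick it polls for top-level HyperSkill and Next (wave change) widgets and checks whether Greedy_BP's DeadSequencer or UsabanModeSequencer is playing.
; Each case calls its own cleanup function, which removes Cutin and Mission widgets; the HyperSkill case calls Mission's Delete instead of RemoveFromParent.
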(event EventBeginPlay)

(event Collision|EventActorBeginOverlap
  (params (OtherActor :type Actor%20Object%20Reference)))

(event EventTick
  (params (DeltaSeconds :type Float%20%28single-precision%29))
  (Utilities|FlowControl|Sequence
    (:then_0
      (bind _foundwidgets (Widget|GetAllWidgetsOfClass "/Game/Throbrave/Widget/HyperSkill.HyperSkill_C" true))
      (for _array_element _foundwidgets
        (Utilities|Casting|CastToHyperSkill _array_element)
        (CallFunction|AddtoHyperSkillWid)))
    (:then_2
      (bind _foundwidgets_2 (Widget|GetAllWidgetsOfClass "/Game/Throbrave/Widget/Next.Next_C" true))
      (for _array_element_2 _foundwidgets_2
        (Utilities|Casting|CastToNext _array_element_2)
        (CallFunction|AddtoWaveChangeWid)))
    (:then_3
      (bind _returnvalue (Actor|GetActorOfClass "/Game/Throbrave/Model/Greedy/BP/Greedy_BP.Greedy_BP_C"))
      (bind _asgreedy_bp (Utilities|Casting|CastToGreedy_BP _returnvalue))
      (if (Audio|Components|Audio|IsPlaying (Variables|/Script/LevelSequence.LevelSequenceActor|GetSequencePlayer (Variables|/Game/Throbrave/Model/Greedy/BP/Greedy_BP.Greedy_BP_C|GetDead%20Sequencer _asgreedy_bp)))
        (CallFunction|StartedBossSequence)
        (elif (Audio|Components|Audio|IsPlaying (Variables|/Script/LevelSequence.LevelSequenceActor|GetSequencePlayer (Variables|/Game/Throbrave/Model/Greedy/BP/Greedy_BP.Greedy_BP_C|GetUsaban%20Mode%20Sequencer _asgreedy_bp)))
          (CallFunction|StartedBossSequence))))))

(fn ConstructionScript)

(fn AddtoHyperSkillWid
  (bind _foundwidgets (Widget|GetAllWidgetsOfClass "/Game/Throbrave/Widget/Mission.Mission_C" true))
  (for _array_element _foundwidgets
    (bind _asmission (Utilities|Casting|CastToMission _array_element))
    (Default|Delete _asmission))
  (bind _foundwidgets_2 (Widget|GetAllWidgetsOfClass "/Game/Throbrave/Widget/Cutin.Cutin_C" true))
  (for _array_element_2 _foundwidgets_2
    (bind _ascutin (Utilities|Casting|CastToCutin _array_element_2))
    (Widget|RemovefromParent _ascutin)))

(fn AddtoWaveChangeWid
  (bind _foundwidgets (Widget|GetAllWidgetsOfClass "/Game/Throbrave/Widget/Mission.Mission_C" true))
  (for _array_element _foundwidgets
    (bind _asmission (Utilities|Casting|CastToMission _array_element))
    (Widget|RemovefromParent _asmission))
  (bind _foundwidgets_2 (Widget|GetAllWidgetsOfClass "/Game/Throbrave/Widget/Cutin.Cutin_C" true))
  (for _array_element_2 _foundwidgets_2
    (bind _ascutin (Utilities|Casting|CastToCutin _array_element_2))
    (Widget|RemovefromParent _ascutin)))

(fn StartedBossSequence
  (bind _foundwidgets (Widget|GetAllWidgetsOfClass "/Game/Throbrave/Widget/Mission.Mission_C" true))
  (for _array_element _foundwidgets
    (bind _asmission (Utilities|Casting|CastToMission _array_element))
    (Widget|RemovefromParent _asmission))
  (bind _foundwidgets_2 (Widget|GetAllWidgetsOfClass "/Game/Throbrave/Widget/Cutin.Cutin_C" true))
  (for _array_element_2 _foundwidgets_2
    (bind _ascutin (Utilities|Casting|CastToCutin _array_element_2))
    (Widget|RemovefromParent _ascutin)))