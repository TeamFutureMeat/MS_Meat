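; Hadou is a projectile Blueprint that flies forward, explodes on contact and deals strong damage to The_Coin actors.
; HadouRotation stores a target and turns the projectile toward it once per call.
; Tick moves it along its local X axis without sweep, destroying it once world X passes a fixed limit.
; Any sphere overlap spawns the NewBomb effect, but only The_Coin takes damage and destroys the projectile.
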(event OnComponentBeginOverlap(Sphere)
  (params (OverlappedComponent :type Primitive%20Component%20Object%20Reference) (OtherActor :type Actor%20Object%20Reference) (OtherComp :type Primitive%20Component%20Object%20Reference) (OtherBodyIndex :type Integer) (bFromSweep :type Boolean) (SweepResult :type Hit%20Result%20Structure%20%28by%20ref%29))
  (Niagara|SpawnSystematLocation "/Game/Throbrave/Particle/PSystemes/NewBomb.NewBomb" (Transformation|GetActorLocation OtherActor))
  (bind _asthe_coin (Utilities|Casting|CastToThe_Coin OtherActor))
  (Default|StrongDamage _asthe_coin 15.0)
  (Actor|DestroyActor))

(event EventBeginPlay)

(event Collision|EventActorBeginOverlap
  (params (OtherActor :type Actor%20Object%20Reference)))

(event EventTick
  (params (DeltaSeconds :type Float%20%28single-precision%29))
  (if (>= 9e+02 (.x (Transformation|GetActorLocation)))
    (Transformation|AddActorLocalOffset "10.000000, 0,0.000000" false false)
    (else
      (Actor|DestroyActor))))

(fn ConstructionScript)

(fn HadouRotation
  (params (ターゲット :type Actor%20Object%20Reference))
  (bind _output_get (Variables|Default|SetEnemy ターゲット))
  (Transformation|SetActorRotation (Math|Rotator|FindLookatRotation (Transformation|GetActorLocation) (Transformation|GetActorLocation _output_get))))