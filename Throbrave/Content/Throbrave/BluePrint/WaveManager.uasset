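; Wave manager actor that runs two enemy waves, then the boss entrance.
; It creates four side spawners at BeginPlay and sets their per-wave spawn caps.
; Tick polls for The_Coin; when none remains in waves one or two, a Next animation and dialogue play before the wave advances.
; Later waves play the DJ entry sequence (same in both IsNoDamage branches), then show boss HP UI, with player buttons released during transitions.
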(event Custom|WaveStart
  (Default|ButtonReBind (Variables|/Game/Throbrave/BluePrint/Player.Player_C|GetButtonWid (Variables|Default|GetPlayer)))
  (CallFunction|SpawnEnemySpawner)
  (Default|ResetEnemyCount (Variables|Default|GetGameInstance)))

(event Custom|CalledNext
  (Math|Integer|IncrementInt (Variables|Default|GetWaveCount)
    (:%20%20
      (Utilities|FlowControl|DoOnce false) ; enters at Reset
    )))

(event Custom|NextFinish
  (Widget|RemovefromParent (stale Custom|NextStart _returnvalue))
  (Variables|Default|SetIsWaveStart true)
  (CallFunction|CommentStart (Variables|Default|GetCommentMode)))

(event Custom|NextStart
  (bind _returnvalue (UserInterface|CreateWidget "/Game/Throbrave/Widget/Next.Next_C"))
  (UserInterface|Viewport|AddtoViewport _returnvalue 0)
  (Class|UserWidget|BindtoAnimationFinished _returnvalue (Variables|/Game/Throbrave/Widget/Next.Next_C|GetNextAnimation _returnvalue) (delegate Custom|NextFinish))
  (Default|ButtonBindRelease (Variables|/Game/Throbrave/BluePrint/Player.Player_C|GetButtonWid (Variables|Default|GetPlayer))))

(event Custom|BossAppearanceAnimEnd
  (bind _pressallwid (Variables|Default|GetPressAllWid))
  (Default|ButtonReBind (Variables|/Game/Throbrave/BluePrint/Player.Player_C|GetButtonWid (Variables|Default|GetPlayer)))
  (bind _asplayer (Utilities|Casting|CastToPlayer (Game|Player|GetPlayerPawn 0)))
  (Variables|/Game/Throbrave/BluePrint/Player.Player_C|SetIsBossPop _asplayer true)
  (Default|BossPop (.AsEnemy%20HP%20UI (Utilities|Casting|CastToEnemyHP_UI (Variables|/Script/Engine.ChildActorComponent|GetChildActor (Variables|/Game/Throbrave/BluePrint/Player.Player_C|GetEnemyHP_UI _asplayer)))))
  (Utilities|IsValid _pressallwid
    (:Is%20Valid
      (UserInterface|Viewport|AddtoViewport _pressallwid 0))))

(event Custom|DialogueAnimEnd
  (bind _dialogue (Variables|Default|GetDialogue))
  (Default|ButtonBindRelease (Variables|/Game/Throbrave/BluePrint/Player.Player_C|GetButtonWid (Variables|Default|GetPlayer)))
  (CallFunction|CalledNext)
  (Class|UserWidget|UnbindfromAnimationFinished _dialogue (Variables|/Game/Throbrave/Widget/Dialogue.Dialogue_C|GetCutoutAnimation _dialogue) (delegate Custom|DialogueAnimEnd)))

(event EventBeginPlay
  (Variables|Default|SetWaveCount 1)
  (CallFunction|SetEnemySpawner)
  (bind _returnvalue (UserInterface|CreateWidget "/Game/Throbrave/Widget/Dialogue.Dialogue_C"))
  (bind _output_get (Variables|Default|SetDialogue _returnvalue))
  (UserInterface|Viewport|AddtoViewport _output_get 0)
  (bind _asplayer (Utilities|Casting|CastToPlayer (Game|Player|GetPlayerPawn 0)))
  (Variables|Default|SetPlayer _asplayer)
  (bind _asmy_game_instance (Utilities|Casting|CastToMyGameInstance (Game|GetGameInstance)))
  (Variables|Default|SetGameInstance _asmy_game_instance))

(event Collision|EventActorBeginOverlap
  (params (OtherActor :type Actor%20Object%20Reference)))

(event EventTick
  (params (DeltaSeconds :type Float%20%28single-precision%29))
  (if (Variables|Default|GetIsWaveStart)
    (Utilities|FlowControl|DoOnce false
      (:Completed
        (CallFunction|WaveStart)
        (Utilities|FlowControl|Delay 1.0)
        (Variables|Default|SetIsWaveStart false)))
    (elif (== (Variables|Default|GetWaveCount) 1)
      (bind _returnvalue (Actor|GetActorOfClass "/Game/Throbrave/Model/TheCoin/BP/The_Coin.The_Coin_C"))
      (Utilities|Casting|CastToThe_Coin _returnvalue
        (:CastFailed
          (Utilities|FlowControl|DoOnce false
            (:Completed
              (CallFunction|NextStart)
              (Variables|Default|SetCommentMode 2)))))
      (elif (== (Variables|Default|GetWaveCount) 2)
        (bind _returnvalue_2 (Actor|GetActorOfClass "/Game/Throbrave/Model/TheCoin/BP/The_Coin.The_Coin_C"))
        (Utilities|Casting|CastToThe_Coin _returnvalue_2
          (:CastFailed
            (Utilities|FlowControl|DoOnce false
              (:Completed
                (CallFunction|NextStart)
                (Variables|Default|SetCommentMode 4)))))))))

(fn ConstructionScript)

(fn SpawnEnemySpawner
  (switch int (Variables|Default|GetWaveCount)
    (:Default
      (if (Variables|/Game/Throbrave/MyGameInstance.MyGameInstance_C|GetIsNoDamage (Variables|Default|GetGameInstance))
        ;[1 1 1] グリーディ登場処理
        (bind _outactor (Sequencer|Player|CreateLevelSequencePlayer "/Game/Throbrave/Sequencer/DJ_Entry_Sequencer.DJ_Entry_Sequencer"))
        (Sequencer|Player|Play (Variables|/Script/LevelSequence.LevelSequenceActor|GetSequencePlayer _outactor) :!class /Script/MovieScene.MovieSceneSequencePlayer)
        (Default|ButtonBindRelease (Variables|/Game/Throbrave/BluePrint/Player.Player_C|GetButtonWid (Variables|Default|GetPlayer)))
        (EventDispatchers|BindEventtoOnFinished (Variables|/Script/LevelSequence.LevelSequenceActor|GetSequencePlayer _outactor) (EventDispatchers|CreateEvent :!event Custom|BossAppearanceAnimEnd))
        (bind _foundwidgets (Widget|GetAllWidgetsOfClass "/Game/Throbrave/Widget/PressAll.PressAll_C" true))
        (for _array_element _foundwidgets
          (bind _aspress_all (Utilities|Casting|CastToPressAll _array_element))
          (bind _output_get (Variables|Default|SetPressAllWid _aspress_all))
          (Widget|RemovefromParent _output_get))
        (else
          ;[1 1 1] DJニギス登場処理
          (bind _outactor_2 (Sequencer|Player|CreateLevelSequencePlayer "/Game/Throbrave/Sequencer/DJ_Entry_Sequencer.DJ_Entry_Sequencer"))
          (Sequencer|Player|Play (Variables|/Script/LevelSequence.LevelSequenceActor|GetSequencePlayer _outactor_2) :!class /Script/MovieScene.MovieSceneSequencePlayer)
          (Default|ButtonBindRelease (Variables|/Game/Throbrave/BluePrint/Player.Player_C|GetButtonWid (Variables|Default|GetPlayer)))
          (EventDispatchers|BindEventtoOnFinished (Variables|/Script/LevelSequence.LevelSequenceActor|GetSequencePlayer _outactor_2) (EventDispatchers|CreateEvent :!event Custom|BossAppearanceAnimEnd))
          (bind _foundwidgets_2 (Widget|GetAllWidgetsOfClass "/Game/Throbrave/Widget/PressAll.PressAll_C" true))
          (for _array_element_2 _foundwidgets_2
            (bind _aspress_all_2 (Utilities|Casting|CastToPressAll _array_element_2))
            (bind _output_get_2 (Variables|Default|SetPressAllWid _aspress_all_2))
            (Widget|RemovefromParent _output_get_2)))))
    (:1
      (for (_array_element_3 _array_index) (Variables|Default|GetSpawnerObjects)
        (Default|SetSpawner _array_element_3 (Utilities|Array|Get(acopy) (Utilities|Array|MakeArray 1.0 2.0 1.0 1.0) _array_index) _array_index)
        (Variables|/Game/Throbrave/BluePrint/EnemySpawner.EnemySpawner_C|SetSpawnCount _array_element_3 0.0)))
    (:2
      (for (_array_element_4 _array_index_2) (Variables|Default|GetSpawnerObjects)
        (Default|SetSpawner _array_element_4 (Utilities|Array|Get(acopy) (Utilities|Array|MakeArray 2.0 2.0 2.0 1.0) _array_index_2) _array_index_2)
        (Variables|/Game/Throbrave/BluePrint/EnemySpawner.EnemySpawner_C|SetSpawnCount _array_element_4 0.0)))))

(fn SetEnemySpawner
  (Utilities|FlowControl|Sequence
    (:then_0
      (bind _returnvalue (Game|SpawnActorfromClass "/Game/Throbrave/BluePrint/EnemySpawner.EnemySpawner_C" (Math|Transform|MakeTransform (Math|Vector|MakeVector 1e+03 1.3e+03 0.0) "0,90.000000, 0" "1,1,1") "Undefined" 0 0))
      (Variables|/Game/Throbrave/BluePrint/EnemySpawner.EnemySpawner_C|SetIsFront _returnvalue true)
      (Variables|/Game/Throbrave/BluePrint/EnemySpawner.EnemySpawner_C|SetIsRight _returnvalue true)
      (Utilities|Array|SetArrayElem (Variables|Default|GetSpawnerObjects) 0 _returnvalue))
    (:then_1
      (bind _returnvalue_2 (Game|SpawnActorfromClass "/Game/Throbrave/BluePrint/EnemySpawner.EnemySpawner_C" (Math|Transform|MakeTransform (Math|Vector|MakeVector 1e+03 -1.3e+03 0.0) "0,-90.000000, 0" "1,1,1") "Undefined" 0 0))
      (Variables|/Game/Throbrave/BluePrint/EnemySpawner.EnemySpawner_C|SetIsFront _returnvalue_2 true)
      (Variables|/Game/Throbrave/BluePrint/EnemySpawner.EnemySpawner_C|SetIsRight _returnvalue_2 false)
      (Utilities|Array|SetArrayElem (Variables|Default|GetSpawnerObjects) 1 _returnvalue_2))
    (:then_2
      (bind _returnvalue_3 (Game|SpawnActorfromClass "/Game/Throbrave/BluePrint/EnemySpawner.EnemySpawner_C" (Math|Transform|MakeTransform (Math|Vector|MakeVector 1e+03 1.3e+03 3e+02) "0,90.000000, 0" "1,1,1") "Undefined" 0 0))
      (Variables|/Game/Throbrave/BluePrint/EnemySpawner.EnemySpawner_C|SetIsFront _returnvalue_3 false)
      (Variables|/Game/Throbrave/BluePrint/EnemySpawner.EnemySpawner_C|SetIsRight _returnvalue_3 true)
      (Utilities|Array|SetArrayElem (Variables|Default|GetSpawnerObjects) 2 _returnvalue_3))
    (:then_3
      (bind _returnvalue_4 (Game|SpawnActorfromClass "/Game/Throbrave/BluePrint/EnemySpawner.EnemySpawner_C" (Math|Transform|MakeTransform (Math|Vector|MakeVector 1e+03 -1.3e+03 3e+02) "0,-90.000000, 0" "1,1,1") "Undefined" 0 0))
      (Variables|/Game/Throbrave/BluePrint/EnemySpawner.EnemySpawner_C|SetIsFront _returnvalue_4 false)
      (Variables|/Game/Throbrave/BluePrint/EnemySpawner.EnemySpawner_C|SetIsRight _returnvalue_4 false)
      (Utilities|Array|SetArrayElem (Variables|Default|GetSpawnerObjects) 3 _returnvalue_4))))

(fn InitEnemySpawner
  (for (_array_element _array_index) (Variables|Default|GetSpawnerObjects)
    (Default|SetSpawner _array_element 0.0 _array_index)))

(fn CommentStart
  (params (CommentMode :type Integer))
  (bind _dialogue (Variables|Default|GetDialogue))
  (Default|ChangeComment _dialogue CommentMode)
  (Class|UserWidget|BindtoAnimationFinished _dialogue (Variables|/Game/Throbrave/Widget/Dialogue.Dialogue_C|GetCutoutAnimation _dialogue) (EventDispatchers|CreateEvent :!event Custom|DialogueAnimEnd)))