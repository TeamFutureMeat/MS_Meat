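; BonusStage is an actor that runs a bonus stage, reacting to the player's left, center and right push inputs.
; On BeginPlay it binds handlers to the Player pawn's three push events, then adds a BonusStageWid to the viewport.
; Center and right pushes each spawn a Point3DWidget at the actor's own transform.
; The left push's spawn call has no class set, so that branch looks unfinished.
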(event Custom|PushLeft
  (bind _returnvalue (Transformation|GetActorTransform))
  (Game|SpawnActorfromClass "/Game/Throbrave/BluePrint/Point3DWidget.Point3DWidget_C" (Math|Transform|MakeTransform (.location _returnvalue) (.rotation _returnvalue) (.scale _returnvalue)) "Undefined" 0 0))

(event Custom|PushCenter
  (Game|SpawnActorfromClass "/Game/Throbrave/BluePrint/Point3DWidget.Point3DWidget_C" (Transformation|GetActorTransform) "Undefined" 0 0))

(event Custom|PushRight
  (Game|SpawnActorfromClass "/Game/Throbrave/BluePrint/Point3DWidget.Point3DWidget_C" (Transformation|GetActorTransform) "Undefined" 0 0))

(event EventBeginPlay
  (bind _asplayer (Utilities|Casting|CastToPlayer (Game|Player|GetPlayerPawn 0)))
  (EventDispatchers|BindEventtoPushLeft _asplayer (delegate Custom|PushLeft))
  (EventDispatchers|BindEventtoPushCenter _asplayer (delegate Custom|PushCenter))
  (EventDispatchers|BindEventtoPushRight _asplayer (delegate Custom|PushRight))
  (bind _returnvalue (UserInterface|CreateWidget "/Game/Throbrave/Widget/BonusStageWid.BonusStageWid_C"))
  (UserInterface|Viewport|AddtoViewport _returnvalue 0))

(event Collision|EventActorBeginOverlap
  (params (OtherActor :type Actor%20Object%20Reference)))

(event EventTick
  (params (DeltaSeconds :type Float%20%28single-precision%29)))

(fn ConstructionScript)