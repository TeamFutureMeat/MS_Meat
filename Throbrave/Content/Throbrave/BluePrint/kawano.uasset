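; Blueprint kawano, an actor that carries two enemy attack widgets on its Attack and Attack1 widget components.
; On BeginPlay it creates two separate EnemyAttack widget instances, stores them, assigns one to each component and makes both visible.
; The WIDGET and WIDGET0 functions each call Attack on their own widget instance, so the two can be triggered independently.
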(event EventBeginPlay
  (bind _attack (Variables|Default|GetAttack))
  (bind _attack1 (Variables|Default|GetAttack1))
  (bind _returnvalue (UserInterface|CreateWidget "/Game/Throbrave/Widget/Enemy/EnemyAttack.EnemyAttack_C"))
  (bind _output_get (Variables|Default|SetEnemyAttack _returnvalue))
  (UserInterface|SetWidget _attack _output_get)
  (Rendering|SetVisibility _attack true false)
  (bind _returnvalue_2 (UserInterface|CreateWidget "/Game/Throbrave/Widget/Enemy/EnemyAttack.EnemyAttack_C"))
  (bind _output_get_2 (Variables|Default|SetEnemyAttack2 _returnvalue_2))
  (UserInterface|SetWidget _attack1 _output_get_2)
  (Rendering|SetVisibility _attack1 true false))

(fn ConstructionScript)

(fn WIDGET
  (Default|Attack (Variables|Default|GetEnemyAttack)))

(fn WIDGET0
  (Default|Attack (Variables|Default|GetEnemyAttack2)))