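; Laser actor for the player's far attack that snaps to the player's BiimSpawner transform when play begins.
; Its capsule overlap checks for The_Coin that is alive and attackable, then spawns a NewBomb effect and applies StrongDamage using the player's FarAttackValue.
; Separate functions nudge the beam's local rotation by a small fixed step per call and destroy the actor, with no callers inside this Blueprint.
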(event OnComponentBeginOverlap(Capsule)
  (params (OverlappedComponent :type Primitive%20Component%20Object%20Reference) (OtherActor :type Actor%20Object%20Reference) (OtherComp :type Primitive%20Component%20Object%20Reference) (OtherBodyIndex :type Integer) (bFromSweep :type Boolean) (SweepResult :type Hit%20Result%20Structure%20%28by%20ref%29))
  (bind _asthe_coin (Utilities|Casting|CastToThe_Coin OtherActor))
  (if (not (or (Variables|/Game/Throbrave/Model/TheCoin/BP/The_Coin.The_Coin_C|GetIsDead _asthe_coin) (not (Variables|/Game/Throbrave/Model/TheCoin/BP/The_Coin.The_Coin_C|GetIsCanAttack _asthe_coin))))
    (Niagara|SpawnSystematLocation "/Game/Throbrave/Particle/PSystemes/NewBomb.NewBomb" (Transformation|GetActorLocation _asthe_coin))
    (Default|StrongDamage _asthe_coin (Variables|/Game/Throbrave/BluePrint/Player.Player_C|GetFarAttackValue (Variables|Default|Getplayer)))))

(event EventBeginPlay
  (bind _asplayer (Utilities|Casting|CastToPlayer (Game|Player|GetPlayerPawn 0)))
  (Variables|Default|Setplayer _asplayer)
  (Transformation|SetActorTransform (Transformation|GetWorldTransform (Variables|/Game/Throbrave/BluePrint/Player.Player_C|GetBiimSpawner (Variables|Default|GetPlayer)))))

(event Collision|EventActorBeginOverlap
  (params (OtherActor :type Actor%20Object%20Reference)))

(event EventTick
  (params (DeltaSeconds :type Float%20%28single-precision%29)))

(fn ConstructionScript)

(fn LazerAddRotation
  (Transformation|AddActorLocalRotation "0,-0.200000, 0" false false))

(fn Destroy
  (Actor|DestroyActor))