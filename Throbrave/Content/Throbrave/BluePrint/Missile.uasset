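; Missile actor Blueprint that sets up homing projectile movement toward a target and spawns a smoke effect.
; On BeginPlay it loops over the Target's sphere components tagged "TargetPoint", assigning each as the homing component, so the last one wins.
; Each iteration also spawns a smoke system at the missile's "SmokePoint" socket location.
; The logic to move the smoke with that socket is disconnected, so the effect is never repositioned.
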(event EventBeginPlay
  (bind _array_element (Utilities|Array|ForEachLoopwithBreak (Actor|GetComponentsbyTag (Variables|Default|GetTarget) "/Script/Engine.SphereComponent" "TargetPoint"))
    (:LoopBody
      (Variables|/Script/Engine.ProjectileMovementComponent|SetHomingTargetComponent (Variables|Default|GetProjectileMovement) _array_element)
      (bind _returnvalue (Niagara|SpawnSystematLocation "/Game/Throbrave/Particle/Smoke/SmokeParticle.SmokeParticle" (Transformation|GetSocketLocation (Variables|Default|GetMissile) "SmokePoint")))
      (Variables|Default|SetSmokeParticle _returnvalue))))

(event Collision|EventActorBeginOverlap
  (params (OtherActor :type Actor%20Object%20Reference)))

(event EventTick
  (params (DeltaSeconds :type Float%20%28single-precision%29)))

(fn ConstructionScript)