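; Enemy actor that attacks periodically and awards the player score when killed.
; On BeginPlay it creates an EnemyAttack widget, picks a randomly offset home position along Y, sets default stats and caches the Player pawn.
; Tick triggers the widget's attack through a frame counter and steps the actor toward home at a fixed, frame-rate-dependent rate.
; Damage reduces life, then adds score and destroys the actor at zero.
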(event EventBeginPlay
  (bind _returnvalue (UserInterface|CreateWidget "/Game/Throbrave/Widget/EnemyAttack.EnemyAttack_C"))
  (bind _output_get (Variables|Default|SetEnemyAttack _returnvalue))
  (UserInterface|Viewport|AddtoViewport _output_get 0)
  (CallFunction|SetDefaultPosition)
  (Utilities|SetDefaultValue)
  (bind _asplayer (Utilities|Casting|CastToPlayer (Game|Player|GetPlayerPawn 0)))
  (Variables|Default|SetPlayer _asplayer))

(event Collision|EventActorBeginOverlap
  (params (OtherActor :type Actor%20Object%20Reference)))

(event EventTick
  (params (DeltaSeconds :type Float%20%28single-precision%29))
  (bind _returnvalue (Transformation|GetActorLocation))
  (bind _returnvalue_2 (Transformation|GetActorLocation))
  (Utilities|FlowControl|Sequence
    (:then_0
      (bind _result (Math|Float|IncrementFloat (Variables|Default|GetAttackCount))
        (:%20%20
          (bind _output_get (Variables|Default|SetAttackCount _result))
          (if (> _output_get (Variables|Default|GetAttackFrequency))
            (Default|Attack (Variables|Default|GetEnemyAttack))
            (Variables|Default|SetAttackCount 0.0)))))
    (:then_1
      (if (not (Math|Vector|Equal(Vector) (Transformation|GetActorLocation) (Variables|Default|GetHomePosition) 0.1))
        (if (< (.y (Transformation|GetActorLocation)) (.y (Variables|Default|GetHomePosition)))
          (Transformation|SetActorLocation (Math|Vector|MakeVector (.x _returnvalue) (+ (.y _returnvalue) 1.0) (.z _returnvalue)) false false)
          (else
            (Transformation|SetActorLocation (Math|Vector|MakeVector (.x _returnvalue_2) (+ (.y _returnvalue_2) -1.0) (.z _returnvalue_2)) false false)))))))

(fn ConstructionScript)

(fn SetDefaultPosition
  (bind _returnvalue (Transformation|GetActorLocation))
  (Variables|Default|SetAddPosition (* (Math|Random|RandomIntegerinRange -3 3) 1e+02))
  (Variables|Default|SetHomePosition (Math|Vector|MakeVector (.x _returnvalue) (+ (.y _returnvalue) (Variables|Default|GetAddPosition)) (.z _returnvalue))))

(fn Damage
  (params (DamageValue :type Float%20%28single-precision%29))
  (bind _output_get (Variables|Default|SetNowLife (- (Variables|Default|GetNowLife) DamageValue)))
  (if (<= _output_get 0.0)
    (Default|AddPlayerScore (Variables|Default|GetPlayer) (Variables|Default|GetScore))
    (Actor|DestroyActor)))