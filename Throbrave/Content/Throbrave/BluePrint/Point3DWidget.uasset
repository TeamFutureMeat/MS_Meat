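; Point3DWidget is an actor that shows a floating score pop-up through a widget component holding a Point widget.
; On BeginPlay it plays the widget's AddScore animation and binds to its finish event.
; When the animation finishes, it adds 100 to the Player pawn's score and destroys itself.
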(event Custom|LeftAnimFinish
  (bind _asplayer (Utilities|Casting|CastToPlayer (Game|Player|GetPlayerPawn 0)))
  (Default|AddPlayerScore _asplayer 100)
  (Actor|DestroyActor))

(event EventBeginPlay
  (bind _point (Variables|Default|GetPoint))
  (bind _returnvalue (UserInterface|GetUserWidgetObject _point))
  (bind _aspoint (Utilities|Casting|CastToPoint _returnvalue))
  (bind _addscore (Variables|/Game/Throbrave/Widget/Point.Point_C|GetAddScore _aspoint))
  (UserInterface|Animation|PlayAnimation _aspoint _addscore 0.0 1 "Forward" 1.0 false)
  (Class|UserWidget|BindtoAnimationFinished _aspoint _addscore (delegate Custom|LeftAnimFinish)))

(event Collision|EventActorBeginOverlap
  (params (OtherActor :type Actor%20Object%20Reference)))

(event EventTick
  (params (DeltaSeconds :type Float%20%28single-precision%29)))

(fn ConstructionScript)