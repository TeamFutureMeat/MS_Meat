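; Enemy spawner that creates movable The_Coin enemies until its spawn cap is reached.
; Tick counts frames against spawner number times spawn frequency, and re-enables spawning whenever the count is below the cap.
; Each coin gets front/back and left/right flags, a shifted Attack component and a default position stepped by spawn count.
; Coins register in the GameInstance's position array by row, and SetSpawner configures cap and spawner number.
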(event Custom|Spawn
  (bind _defaultenemyposition (Variables|Default|GetDefaultEnemyPosition))
  (bind _spawncount (Variables|Default|GetSpawnCount))
  (bind _gameinstance (Variables|Default|GetGameInstance))
  (bind _returnvalue (* _spawncount 2e+02))
  (bind _returnvalue_2 (Game|SpawnActorfromClass "/Game/Throbrave/Model/TheCoin/BP/The_Coin.The_Coin_C" (Transformation|GetActorTransform) "Undefined" 0 0))
  (Variables|/Game/Throbrave/Model/TheCoin/BP/The_Coin.The_Coin_C|SetIsCanMove _returnvalue_2 true)
  (if (Variables|Default|GetIsFront)
    (Variables|/Game/Throbrave/Model/TheCoin/BP/The_Coin.The_Coin_C|SetIsFront _returnvalue_2 true)
    (Transformation|SetWorldLocation (Variables|/Game/Throbrave/Model/TheCoin/BP/The_Coin.The_Coin_C|GetAttack _returnvalue_2) (Math|Vector|MakeVector (+ (.x (Transformation|GetWorldLocation (Variables|/Game/Throbrave/Model/TheCoin/BP/The_Coin.The_Coin_C|GetAttack _returnvalue_2))) -1.5e+02) (.y (Transformation|GetWorldLocation (Variables|/Game/Throbrave/Model/TheCoin/BP/The_Coin.The_Coin_C|GetAttack _returnvalue_2))) (.z (Transformation|GetWorldLocation (Variables|/Game/Throbrave/Model/TheCoin/BP/The_Coin.The_Coin_C|GetAttack _returnvalue_2)))) false false)
    (Default|SetEnemyPositionArray _gameinstance false _returnvalue_2)
    (if (Variables|Default|GetIsRight)
      (Variables|/Game/Throbrave/Model/TheCoin/BP/The_Coin.The_Coin_C|SetIsRight _returnvalue_2 true :!label _label)
      (Default|SetDefaultPosition _returnvalue_2 (+ (* -1 _defaultenemyposition) _returnvalue))
      (else
        (Variables|/Game/Throbrave/Model/TheCoin/BP/The_Coin.The_Coin_C|SetIsRight _returnvalue_2 false :!label _label_2)
        (Default|SetDefaultPosition _returnvalue_2 (- _defaultenemyposition _returnvalue))))
    (else
      (Transformation|SetWorldLocation (Variables|/Game/Throbrave/Model/TheCoin/BP/The_Coin.The_Coin_C|GetAttack _returnvalue_2) (Math|Vector|MakeVector (+ (.x (Transformation|GetWorldLocation (Variables|/Game/Throbrave/Model/TheCoin/BP/The_Coin.The_Coin_C|GetAttack _returnvalue_2))) -5e+02) (.y (Transformation|GetWorldLocation (Variables|/Game/Throbrave/Model/TheCoin/BP/The_Coin.The_Coin_C|GetAttack _returnvalue_2))) (.z (Transformation|GetWorldLocation (Variables|/Game/Throbrave/Model/TheCoin/BP/The_Coin.The_Coin_C|GetAttack _returnvalue_2)))) false false)
      (Default|SetEnemyPositionArray _gameinstance true _returnvalue_2)
      (if (Variables|Default|GetIsRight)
        (goto _label)
        (else
          (goto _label_2)))))
  (Default|CallEnemySpawn)
  (bind _result (Math|Float|IncrementFloat (Variables|Default|GetSpawnCount))
    (:%20%20
      (if (>= _result (Variables|Default|GetEnemySpawnMax))
        (Variables|Default|SetIsSpawn false)))))

(event Custom|SetSpawner
  (params (EnemySpawnMax :type Float%20%28single-precision%29) (SpawnNumber :type Integer))
  (Variables|Default|SetEnemySpawnMax EnemySpawnMax)
  (Variables|Default|SetSpawnerNumber SpawnNumber))

(event EventBeginPlay
  (bind _asmy_game_instance (Utilities|Casting|CastToMyGameInstance (Game|GetGameInstance)))
  (Variables|Default|SetGameInstance _asmy_game_instance))

(event Collision|EventActorBeginOverlap
  (params (OtherActor :type Actor%20Object%20Reference)))

(event EventTick
  (params (DeltaSeconds :type Float%20%28single-precision%29))
  (if (Variables|Default|GetIsSpawn)
    (bind _result (Math|Float|IncrementFloat (Variables|Default|GetSpawnerTime))
      (:%20%20
        (bind _output_get (Variables|Default|SetSpawnerTime _result))
        (if (> _output_get (* (Variables|Default|GetSpawnerNumber) (Variables|Default|GetSpawnFrequency)))
          (CallFunction|Spawn)
          (Variables|Default|SetSpawnerTime 0.0))))
    (elif (< (Variables|Default|GetSpawnCount) (Variables|Default|GetEnemySpawnMax))
      (Variables|Default|SetIsSpawn true))))

(fn ConstructionScript)