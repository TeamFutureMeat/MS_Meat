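; DJ_Dead is the DJニギス enemy, with hit points, a damage event that calls a dispatcher, and an IsAlive flag.
; Tick drives a DoOnce-and-Delay attack loop that picks random timer-scheduled attack sequences.
; Below 70% health, sequences add Scratch, and a one-time Tempo Up doubles attack damage.
; Attacks only set a Damage value and print their names; the health-bar widget creation is unconnected.
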(event Custom|DJ_Damage
  (params (DamageNum :type Float%20%28single-precision%29))
  (Variables|Default|SetNowHitPoint (- (Variables|Default|GetNowHitPoint) DamageNum))
  (Default|CallDJDamageDispatcher))

(event EventTick
  (params (DeltaSeconds :type Float%20%28single-precision%29))
  (Utilities|FlowControl|Sequence
    (:then_0
      (Utilities|DJAttackRoutine))
    (:then_1
      (if (< (Variables|Default|GetNowHitPoint) 0.0)
        (Variables|Default|SetIsAlive false)))))

(event EventBeginPlay
  (bind _output_get (Variables|Default|SetMaxHitPoint 1e+02))
  (Variables|Default|SetNowHitPoint _output_get)
  (Variables|Default|SetAttackDamage 15.0)
  (Variables|Default|SetAttackWaitTime 5.0)
  (Variables|Default|SetDJ_ULT false)
  (Variables|Default|SetAttackNum 3.0)
  (Variables|Default|SetIsAlive true))

(fn ConstructionScript)

(fn DJAttackPaternTAIATARI
  (Variables|Default|SetDamage (* (Variables|Default|GetAttackDamage) 1.0))
  (Development|PrintString "DJニギス-体当たり"))

(fn DJAttackPaternONPA
  (Variables|Default|SetDamage (* (Variables|Default|GetAttackDamage) 1.2))
  (Development|PrintString "DJニギス-音波"))

(fn DJAttackPaternSUKURATTI
  (Variables|Default|SetDamage (* (Variables|Default|GetAttackDamage) 1.5))
  (Development|PrintString "DJニギス-スクラッチ"))

(fn DJAttackPaternTENPOAPPU
  (Variables|Default|SetAttackDamage (* (Variables|Default|GetAttackDamage) 2.0))
  (Variables|Default|SetDamage (* (Variables|Default|GetAttackDamage) 2.0))
  (Development|PrintString "DJニギス-テンポアップ"))

(fn DJRoutine1
  (bind _output_get (Variables|Default|Setrand (Math|Random|RandomInteger 4)))
  (Development|PrintString (Utilities|String|ToString(Integer) _output_get))
  (switch int _output_get
    (:0
      (Utilities|Time|SetTimerbyFunctionName 0 "DJ_AttackPatern_TAIATARI" (Variables|Default|GetAttackWaitTime))
      (bind _returnvalue (Utilities|Time|SetTimerbyFunctionName 0 "DJ_AttackPatern_ONPA" (* (Variables|Default|GetAttackWaitTime) 2.0))))
    (:1
      (Utilities|Time|SetTimerbyFunctionName 0 "DJ_AttackPatern_TAIATARI" (Variables|Default|GetAttackWaitTime))
      (bind _returnvalue_2 (Utilities|Time|SetTimerbyFunctionName 0 "DJ_AttackPatern_TAIATARI" (* (Variables|Default|GetAttackWaitTime) 2.0))))
    (:2
      (Utilities|Time|SetTimerbyFunctionName 0 "DJ_AttackPatern_ONPA" (Variables|Default|GetAttackWaitTime))
      (bind _returnvalue_3 (Utilities|Time|SetTimerbyFunctionName 0 "DJ_AttackPatern_ONPA" (* (Variables|Default|GetAttackWaitTime) 2.0))))
    (:3
      (Utilities|Time|SetTimerbyFunctionName 0 "DJ_AttackPatern_ONPA" (Variables|Default|GetAttackWaitTime))
      (bind _returnvalue_4 (Utilities|Time|SetTimerbyFunctionName 0 "DJ_AttackPatern_TAIATARI" (* (Variables|Default|GetAttackWaitTime) 2.0)))))
  (return (Utilities|Array|MakeArray _returnvalue _returnvalue_2 _returnvalue_3 _returnvalue_4)))

(fn DJRoutine2
  (bind _output_get (Variables|Default|Setrand (Math|Random|RandomInteger 5)))
  (Development|PrintString (Utilities|String|ToString(Integer) _output_get))
  (switch int _output_get
    (:0
      (Utilities|Time|SetTimerbyFunctionName 0 "DJ_AttackPatern_TAIATARI" (Variables|Default|GetAttackWaitTime))
      (Utilities|Time|SetTimerbyFunctionName 0 "DJ_AttackPatern_ONPA" (* (Variables|Default|GetAttackWaitTime) 2.0))
      (bind _returnvalue (Utilities|Time|SetTimerbyFunctionName 0 "DJ_AttackPatern_SUKURATTI" (* (Variables|Default|GetAttackWaitTime) 3.0))))
    (:1
      (Utilities|Time|SetTimerbyFunctionName 0 "DJ_AttackPatern_TAIATARI" (Variables|Default|GetAttackWaitTime))
      (Utilities|Time|SetTimerbyFunctionName 0 "DJ_AttackPatern_SUKURATTI" (* (Variables|Default|GetAttackWaitTime) 2.0))
      (bind _returnvalue_2 (Utilities|Time|SetTimerbyFunctionName 0 "DJ_AttackPatern_ONPA" (* (Variables|Default|GetAttackWaitTime) 3.0))))
    (:2
      (Utilities|Time|SetTimerbyFunctionName 0 "DJ_AttackPatern_SUKURATTI" (Variables|Default|GetAttackWaitTime))
      (Utilities|Time|SetTimerbyFunctionName 0 "DJ_AttackPatern_TAIATARI" (* (Variables|Default|GetAttackWaitTime) 2.0))
      (bind _returnvalue_3 (Utilities|Time|SetTimerbyFunctionName 0 "DJ_AttackPatern_ONPA" (* (Variables|Default|GetAttackWaitTime) 3.0))))
    (:3
      (Utilities|Time|SetTimerbyFunctionName 0 "DJ_AttackPatern_ONPA" (Variables|Default|GetAttackWaitTime))
      (Utilities|Time|SetTimerbyFunctionName 0 "DJ_AttackPatern_SUKURATTI" (* (Variables|Default|GetAttackWaitTime) 2.0))
      (bind _returnvalue_4 (Utilities|Time|SetTimerbyFunctionName 0 "DJ_AttackPatern_TAIATARI" (* (Variables|Default|GetAttackWaitTime) 3.0))))
    (:4
      (Utilities|Time|SetTimerbyFunctionName 0 "DJ_AttackPatern_SUKURATTI" (Variables|Default|GetAttackWaitTime))
      (Utilities|Time|SetTimerbyFunctionName 0 "DJ_AttackPatern_TAIATARI" (* (Variables|Default|GetAttackWaitTime) 2.0))
      (bind _returnvalue_5 (Utilities|Time|SetTimerbyFunctionName 0 "DJ_AttackPatern_SUKURATTI" (* (Variables|Default|GetAttackWaitTime) 3.0)))))
  (return (Utilities|Array|MakeArray _returnvalue _returnvalue_2 _returnvalue_3 _returnvalue_4 _returnvalue_5)))

(fn DJRoutine3
  (if (not (Variables|Default|GetDJ_ULT))
    (Variables|Default|SetDJ_ULT true)
    (Utilities|Time|SetTimerbyFunctionName 0 "DJ_AttackPatern_TENPOAPPU" (Variables|Default|GetAttackWaitTime))))