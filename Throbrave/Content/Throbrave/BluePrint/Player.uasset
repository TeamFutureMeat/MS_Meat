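; Player Blueprint managing HP, score, ultimate gauge, game-over/continue flow and three-direction button input with simultaneous-press detection.
; Button widget events charge the ultimate into HyperSkill and count just guards; three guards start a roulette and timed Zone buff, fading video materials onto the glass.
; Tick drives score-tier aura and widget changes, plus boss HP shutter opening with BGM crossfade.
; Includes debug keys and a provisional timing-stop slot roulette.
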(event Custom|GuardSuccess
  (Utilities|FlowControl|Gate false :!label _label
    (:Exit
      (bind _result (Math|Float|IncrementFloat (Variables|Default|GetGuardCount))
        (:%20%20
          (bind _output_get (Variables|Default|SetGuardCount _result))
          (if (>= _output_get 3.0)
            (Utilities|FlowControl|Sequence
              (:then_0
                (goto _label Close))
              (:then_1
                (bind _asroulette_ui (Utilities|Casting|CastToRoulette_UI (Variables|/Script/Engine.ChildActorComponent|GetChildActor (Variables|Default|GetRoulette_UI))))
                (Default|RouletteStart _asroulette_ui)
                (Variables|Default|SetGuardCount 0.0)
                ;[1 1 1] Zoneの切り替え
                (Utilities|InitZoneMaterial)
                (Utilities|FlowControl|Delay 3.5)
                (Rendering|Material|SetMaterial (Variables|Default|GetLeftGlass) 0 "/Game/Movies/ZoneMediaPlayer_Video_Mat.ZoneMediaPlayer_Video_Mat")
                (Rendering|Material|SetMaterial (Variables|Default|GetRightGlass) 0 "/Game/Movies/ZoneMediaPlayer_Video_Mat.ZoneMediaPlayer_Video_Mat")
                (bind _zone_type1 (CallFunction|Zone (Variables|Default|Getplayer_buff_type)))
                (bind _新規track_0 (Timeline|Opacity_TimeLine PlayFromStart)
                  (:Update
                    (Rendering|Material|SetScalarParameterValueonMaterials (Variables|Default|GetLeftGlass) "ZoneA" _新規track_0)
                    (Rendering|Material|SetScalarParameterValueonMaterials (Variables|Default|GetRightGlass) "ZoneA" _新規track_0)
                    (Utilities|DelayMacro _zone_type1
                      (:Completed
                        (bind _新規track_0_2 (Timeline|opacity_TimeLine2 PlayFromStart)
                          (:Update
                            (Rendering|Material|SetScalarParameterValueonMaterials (Variables|Default|GetLeftGlass) "ZoneA" _新規track_0_2)
                            (Rendering|Material|SetScalarParameterValueonMaterials (Variables|Default|GetRightGlass) "ZoneA" _新規track_0_2)
                            (goto _label Open)))))))))))))))

(event Custom|FadeAnimEnd
  (Utilities|FlowControl|Delay 2.0)
  (CallFunction|ShowContinue))

(event Custom|Damage
  (params (DamageValue :type Float%20%28single-precision%29))
  (CallFunction|PlayerDamage DamageValue)
  (CallFunction|GameOver (delegate Custom|FadeAnimEnd)))

(event Custom|PressButtonEvent
  (if (> 1e+02 (Variables|Default|GetPlayerUlt))
    (Variables|Default|SetPlayerUlt (+ (Variables|Default|GetPlayerUlt) 5.0))
    (if (>= (Variables|Default|GetPlayerUlt) 1e+02)
      (Utilities|FlowControl|DoOnce false
        (:Completed
          (CallFunction|UltMaxWidjet))))))

(event Custom|BossPop
  (bind _enemyhp_1206_enemyhp_shutter_l (Variables|Default|GetEnemyHP_1206_EnemyHP_Shutter_L))
  (bind _enemyhp_1206_enemyhp_shutter_r (Variables|Default|GetEnemyHP_1206_EnemyHP_Shutter_R))
  (bind _returnvalue (Transformation|GetWorldLocation _enemyhp_1206_enemyhp_shutter_r))
  (bind _returnvalue_2 (Transformation|GetWorldScale _enemyhp_1206_enemyhp_shutter_r))
  (bind _returnvalue_3 (Transformation|GetWorldLocation _enemyhp_1206_enemyhp_shutter_l))
  (bind _returnvalue_4 (Transformation|GetWorldScale _enemyhp_1206_enemyhp_shutter_l))
  (bind _returnvalue_5 (- (.y _returnvalue_3) 1.0))
  (bind _returnvalue_6 (+ (.y _returnvalue) 1.0))
  ;[1 1 1] ボスのHPバーが開くところ
  (Utilities|FlowControl|Sequence
    (:then_0
      (Utilities|FlowControl|DoOnce false :!label _label
        (:Completed
          (Transformation|SetWorldLocation _enemyhp_1206_enemyhp_shutter_l (Math|Vector|MakeVector (.x _returnvalue_3) _returnvalue_5 (.z _returnvalue_3)) false false)
          (Transformation|SetWorldScale3D _enemyhp_1206_enemyhp_shutter_l (Math|Vector|MakeVector (.x _returnvalue_4) (- (.y _returnvalue_4) 0.025) (.z _returnvalue_4)))
          (if (>= _returnvalue_5 -3.8e+02)
            (goto _label Reset)))))
    (:then_1
      (Utilities|FlowControl|DoOnce false :!label _label_2
        (:Completed
          (Transformation|SetWorldLocation _enemyhp_1206_enemyhp_shutter_r (Math|Vector|MakeVector (.x _returnvalue) _returnvalue_6 (.z _returnvalue)) false false)
          (Transformation|SetWorldScale3D _enemyhp_1206_enemyhp_shutter_r (Math|Vector|MakeVector (.x _returnvalue_2) (- (.y _returnvalue_2) 0.025) (.z _returnvalue_2)))
          (if (<= _returnvalue_6 3.8e+02)
            (goto _label_2 Reset)))))))

(event Custom|UltBurstEvent
  (Variables|Default|SetPlayerUlt 0.0)
  (Default|ButtonBindRelease (Variables|Default|GetButtonWid))
  (CallFunction|HyperSkill)
  (Utilities|FlowControl|DoOnce false) ; enters at Reset
)

(event Custom|ScoreTimeLineEvent
  (bind _score_1206_score_frame (Variables|Default|GetScore_1206_Score_frame))
  (bind _returnvalue (Transformation|GetWorldLocation _score_1206_score_frame))
  (bind _新規track_0 (Timeline|タイムライン_0 PlayFromStart)
    (:Update
      (Transformation|SetWorldLocation _score_1206_score_frame (Math|Vector|MakeVector (.x _returnvalue) (.y _returnvalue) (+ _新規track_0 (Variables|Default|GetScorePositionZ))) false false))))

(event EventBeginPlay
  (Utilities|InitStatus)
  (Utilities|InitZoneMaterial)
  (CallFunction|CastButtonWid (delegate Custom|GuardSuccess))
  (bind _asbutton (Utilities|Casting|CastToButton (Utilities|GetButtonBP)))
  (Variables|Default|SetButtonWid _asbutton)
  (EventDispatchers|BindEventtoUltBurst _asbutton (delegate Custom|UltBurstEvent))
  (bind _asscore (Utilities|Casting|CastToScore (Utilities|GetScoreBP)))
  (Default|SetViewScore _asscore (Variables|Default|GetPlayer_Score))
  (EventDispatchers|AssignPressButton _asbutton (delegate Custom|PressButtonEvent))
  (bind _returnvalue (UserInterface|CreateWidget "/Game/Throbrave/Widget/ScorePoint.ScorePoint_C"))
  (UserInterface|SetWidget (Variables|Default|GetTortalScoreWidget) _returnvalue)
  (Utilities|SetAudio))

(event Collision|EventActorBeginOverlap
  (params (OtherActor :type Actor%20Object%20Reference)))

(event EventTick
  (params (DeltaSeconds :type Float%20%28single-precision%29))
  (Utilities|FlowControl|Sequence
    (:then_0
      (Utilities|ChangeColorMacro))
    (:then_1
      (if (Variables|Default|GetIsBossPop)
        (CallFunction|BossPop)
        (Utilities|FlowControl|DoOnce false
          (:Completed
            (Audio|Components|Audio|FadeOut (Variables|Default|GetGameBGM) 1.0 0.0 "Linear" :!class /Script/Engine.AudioComponent)
            (Audio|Components|Audio|FadeIn (Variables|Default|GetDJBGM) 1.0 1.0 0.0 "Linear" :!class /Script/Engine.AudioComponent)))))))

(event Input|KeyboardEvents|Down
  (params (Key :type Key%20Structure :default "None"))
  (:Pressed
    (Utilities|FlowControl|Gate false :!label _label
      (:Exit
        (bind _result (Math|Float|IncrementFloat (Variables|Default|GetGuardCount))
          (:%20%20
            (bind _output_get (Variables|Default|SetGuardCount _result))
            (if (>= _output_get 3.0)
              (Utilities|FlowControl|Sequence
                (:then_0
                  (goto _label Close))
                (:then_1
                  (bind _asroulette_ui (Utilities|Casting|CastToRoulette_UI (Variables|/Script/Engine.ChildActorComponent|GetChildActor (Variables|Default|GetRoulette_UI))))
                  (Default|RouletteStart _asroulette_ui)
                  (Variables|Default|SetGuardCount 0.0)
                  ;[1 1 1] Zoneの切り替え
                  (Utilities|InitZoneMaterial)
                  (Utilities|FlowControl|Delay 3.5)
                  (Rendering|Material|SetMaterial (Variables|Default|GetLeftGlass) 0 "/Game/Movies/ZoneMediaPlayer_Video_Mat.ZoneMediaPlayer_Video_Mat")
                  (Rendering|Material|SetMaterial (Variables|Default|GetRightGlass) 0 "/Game/Movies/ZoneMediaPlayer_Video_Mat.ZoneMediaPlayer_Video_Mat")
                  (bind _zone_type1 (CallFunction|Zone (Variables|Default|Getplayer_buff_type)))
                  (bind _新規track_0 (Timeline|Opacity_TimeLine PlayFromStart)
                    (:Update
                      (Rendering|Material|SetScalarParameterValueonMaterials (Variables|Default|GetLeftGlass) "ZoneA" _新規track_0)
                      (Rendering|Material|SetScalarParameterValueonMaterials (Variables|Default|GetRightGlass) "ZoneA" _新規track_0)
                      (Utilities|DelayMacro _zone_type1
                        (:Completed
                          (bind _新規track_0_2 (Timeline|opacity_TimeLine2 PlayFromStart)
                            (:Update
                              (Rendering|Material|SetScalarParameterValueonMaterials (Variables|Default|GetLeftGlass) "ZoneA" _新規track_0_2)
                              (Rendering|Material|SetScalarParameterValueonMaterials (Variables|Default|GetRightGlass) "ZoneA" _新規track_0_2)
                              (goto _label Open))))))))))))))))

(event Input|KeyboardEvents|Up
  (params (Key :type Key%20Structure :default "None"))
  (:Pressed
    (if (Utilities|SimultaneousPushC)
      (Default|CallPushSimultaneous)
      (else
        (Default|CallPushCenter)
        (CallFunction|PushNavi 1)))))

(event Input|KeyboardEvents|Right
  (params (Key :type Key%20Structure :default "None"))
  (:Pressed
    (if (Utilities|SimultaneousPushR)
      (Default|CallPushSimultaneous)
      (else
        (Default|CallPushRight)
        (CallFunction|PushNavi 2))))
  (:Released
    (Default|CallPushRightReleased)))

(event Input|KeyboardEvents|Enter
  (params (Key :type Key%20Structure :default "None"))
  ;[1 1 1] デバッグ用
  (:Pressed
    (bind _asbutton (Utilities|Casting|CastToButton (Utilities|GetButtonBP)))
    (Variables|/Game/Throbrave/Widget/Button.Button_C|SetSkillGauge_A _asbutton 1.0)
    (Variables|/Game/Throbrave/Widget/Button.Button_C|SetSkillGauge_C _asbutton 1.0)
    (Variables|Default|SetPlayerUlt 1e+02)))

(event Input|KeyboardEvents|M
  (params (Key :type Key%20Structure :default "None"))
  ;[1 1 1] デバッグ用
  (:Pressed
    (bind _returnvalue (Actor|GetActorOfClass "/Game/Throbrave/Model/DJ/BP/DJ.DJ_C"))
    (bind _asdj (Utilities|Casting|CastToDJ _returnvalue))
    (Default|DJDebugAttack _asdj)))

(event Input|KeyboardEvents|A
  (params (Key :type Key%20Structure :default "None"))
  ;[1 1 1] 目押しスロット回転(仮置)
  (:Pressed
    (Utilities|FlowControl|DoOnce false
      (:Completed
        (bind _returnvalue (UserInterface|CreateWidget "/Game/Throbrave/Widget/RouletteNERAE.RouletteNERAE_C"))
        (bind _output_get (Variables|Default|SetNERAERoulette _returnvalue))
        (UserInterface|Viewport|AddtoViewport _output_get 0)
        (Default|NERAE _output_get)))))

(event Input|KeyboardEvents|D
  (params (Key :type Key%20Structure :default "None"))
  ;[1 1 1] 目押しスロット回転(仮置)
  (:Pressed
    (Default|StopRoulette (Variables|Default|GetNERAERoulette))
    (if (Variables|/Game/Throbrave/Widget/RouletteNERAE.RouletteNERAE_C|GetRouletteStop (Variables|Default|GetNERAERoulette))
      (Utilities|FlowControl|Delay 1.0)
      (Widget|RemovefromParent (Variables|Default|GetNERAERoulette))
      (Utilities|FlowControl|DoOnce false) ; enters at Reset
    )))

(event Input|KeyboardEvents|Left
  (params (Key :type Key%20Structure :default "None"))
  (:Pressed
    (if (Utilities|SimultaneousPushL)
      (Default|CallPushSimultaneous)
      (else
        (Default|CallPushLeft)
        (CallFunction|PushNavi)))))

(fn ConstructionScript)

(fn AddPlayerScore
  (params (AddScoreValue :type Integer))
  (bind _output_get (Variables|Default|SetPlayer_Score (+ AddScoreValue (Variables|Default|GetPlayer_Score))))
  (if (<= _output_get 99999999)
    _
    (else
      (Variables|Default|SetPlayer_Score 99999999)))
  (bind _asscore (Utilities|Casting|CastToScore (Utilities|GetScoreBP)))
  (Default|SetNumbers _asscore (Variables|Default|GetPlayer_Score)))

(fn GameOver
  (params (Delegate :type Delegate))
  (if (<= (Variables|Default|GetPlayerHP) 0.0)
    (if (not (Variables|Default|GetIsDead))
      (Variables|Default|SetIsDead true)
      (bind _returnvalue (UserInterface|CreateWidget "/Game/Throbrave/Widget/GameOver.GameOver_C"))
      (UserInterface|Viewport|AddtoViewport _returnvalue 2)
      (UserInterface|Animation|PlayAnimation _returnvalue (Variables|/Game/Throbrave/Widget/GameOver.GameOver_C|GetFade _returnvalue) 0.0 1 "Forward" 1.0 false)
      (UserInterface|Animation|PlayAnimation _returnvalue (Variables|/Game/Throbrave/Widget/GameOver.GameOver_C|GetText _returnvalue) 0.0 1 "Forward" 1.0 false)
      (Class|UserWidget|BindtoAnimationFinished _returnvalue (Variables|/Game/Throbrave/Widget/GameOver.GameOver_C|GetFade _returnvalue) Delegate)
      (Default|ButtonBindRelease (Variables|Default|GetButtonWid))
      (Audio|Components|Audio|FadeOut (Variables|Default|GetGameBGM) 1.0 0.0 "Linear" :!class /Script/Engine.AudioComponent)
      (return))))

(fn ShowResult
  (bind _returnvalue (UserInterface|CreateWidget "/Game/Throbrave/Widget/Result.Result_C"))
  (UserInterface|Viewport|AddtoViewport _returnvalue 2)
  (Game|SetGamePaused true))

(fn CastButtonWid
  (params (Delegate :type Delegate%20%28by%20ref%29))
  (bind _asbutton_ui (Utilities|Casting|CastToButton_UI (Variables|/Script/Engine.ChildActorComponent|GetChildActor (Variables|Default|GetButton_UI))))
  (bind _asbutton (Utilities|Casting|CastToButton (UserInterface|GetUserWidgetObject (Variables|/Game/Throbrave/BluePrint/UI/Button_UI.Button_UI_C|GetButtonWid _asbutton_ui))))
  (EventDispatchers|BindEventtoJustGuard _asbutton Delegate))

(fn PlayerDamage
  (params (DamageValue :type Float%20%28single-precision%29))
  (Utilities|FlowControl|Sequence
    (:then_1
      (if (< 0.0 (Variables|Default|GetPlayerHP))
        (Variables|Default|SetPlayerHP (- (Variables|Default|GetPlayerHP) DamageValue))))))

(fn PressButton
  (if (> 1e+02 (Variables|Default|GetPlayerUlt))
    (Variables|Default|SetPlayerUlt (+ (Variables|Default|GetPlayerUlt) 1e+01))))

(fn HyperSkill
  (bind _returnvalue (UserInterface|CreateWidget "/Game/Throbrave/Widget/HyperSkill.HyperSkill_C"))
  (UserInterface|Viewport|AddtoViewport _returnvalue 0)
  (Default|UltBurst _returnvalue)
  (Widget|RemovefromParent (Variables|Default|GetPressAllWid)))

(fn Zone
  (params (Zone_type :type Integer))
  (bind _buttonwid (Variables|Default|GetButtonWid))
  (switch int Zone_type
    (:0
      (Media|MediaPlayer|OpenSource (Variables|Default|GetZoneMedia) "/Game/Movies/main_Attack.main_Attack")
      (Variables|Default|SetFarAttackValue 18.0)
      (Variables|Default|SetNearAttackValue 24.0))
    (:1
      (Media|MediaPlayer|OpenSource (Variables|Default|GetZoneMedia) "/Game/Movies/main_Cool.main_Cool")
      (Variables|/Game/Throbrave/Widget/Button.Button_C|SetCoolTime_A _buttonwid 1)
      (Variables|/Game/Throbrave/Widget/Button.Button_C|SetCoolTime_C _buttonwid 3))
    (:2
      (Media|MediaPlayer|OpenSource (Variables|Default|GetZoneMedia) "/Game/Movies/main_Gage.main_Gage")
      (Variables|/Game/Throbrave/Widget/Button.Button_C|SetAddGaugeValue_A _buttonwid 0.15)
      (Variables|/Game/Throbrave/Widget/Button.Button_C|SetAddGaugeValue_C _buttonwid 0.15))
    (:3
      (Media|MediaPlayer|OpenSource (Variables|Default|GetZoneMedia) "/Game/Movies/main_Mission.main_Mission")
      (bind _returnvalue (UserInterface|CreateWidget "/Game/Throbrave/Widget/Mission.Mission_C"))
      (UserInterface|Viewport|AddtoViewport _returnvalue 0)))
  (return Zone_type))

(fn UltMaxWidjet
  (bind _buttonwid (Variables|Default|GetButtonWid))
  (bind _returnvalue (UserInterface|CreateWidget "/Game/Throbrave/Widget/PressAll.PressAll_C"))
  (bind _output_get (Variables|Default|SetPressAllWid _returnvalue))
  (UserInterface|Viewport|AddtoViewport _output_get 0)
  (Default|PlayVoice _output_get)
  (Variables|/Game/Throbrave/Widget/Button.Button_C|SetSkillGauge_A _buttonwid 0.0)
  (Variables|/Game/Throbrave/Widget/Button.Button_C|SetSkillGauge_C _buttonwid 0.0)
  (Audio|PlaySound2D "/Game/Throbrave/Sound/SE/BtteleUI/BU_SpecialSkill_Charge/BU_SpecialSkill_Charge_Cue.BU_SpecialSkill_Charge_Cue" 1.0 1.0 0.0 0 0))

(fn PushNavi
  (params (Selection :type Integer))
  (bind _foundwidgets (Widget|GetAllWidgetsOfClass "/Game/Throbrave/Widget/Navi.Navi_C" true))
  (for _array_element _foundwidgets
    (Default|PushOrder _array_element Selection)))

(fn ScoreAnimation
  (Transformation|AddActorLocalOffset (Math|Vector|MakeVector 0.0 0.0 0.0) false false))

(fn ShowContinue
  (bind _returnvalue (UserInterface|CreateWidget "/Game/Throbrave/Widget/Continue.Continue_C"))
  (UserInterface|Viewport|AddtoViewport _returnvalue 3)
  (Game|SetGamePaused true)
  (Variables|Default|SetPlayerHP (Variables|Default|GetPlayerMaxHP)))

(fn StopAllBGM
  (Audio|Components|Audio|Stop (Variables|Default|GetGameBGM))
  (Audio|Components|Audio|Stop (Variables|Default|GetDJBGM)))