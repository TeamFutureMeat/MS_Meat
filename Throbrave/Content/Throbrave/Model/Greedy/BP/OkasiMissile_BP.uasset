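; OkasiMissile_BP is a missile projectile actor in the Greedy folder, aimed at a target actor.
; On BeginPlay it hands its projectile movement, target and "TargetPoint" tag to ProjectileComponentBP, and attaches a smoke particle system at SmokePoint.
; Tick polls the component's HitTarget flag and destroys the missile once it is set, leaving targeting and hit detection to that component.
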(event EventBeginPlay
  (Default|ProjectileComponentInitialize (Variables|Default|GetProjectileComponent_BP) (Variables|Default|GetProjectileMovement) (Variables|Default|GetTarget) "TargetPoint" self)
  (Niagara|SpawnSystemAttached "/Game/Throbrave/Particle/Smoke/SmokeParticle.SmokeParticle" (Variables|Default|GetSmokePoint) "None" "0, 0, 0" "0, 0, 0" "KeepRelativeOffset" true))

(event Collision|EventActorBeginOverlap
  (params (OtherActor :type Actor%20Object%20Reference)))

(event EventTick
  (params (DeltaSeconds :type Float%20%28single-precision%29))
  (if (Variables|/Game/Throbrave/BluePrint/ProjectileComponent_BP.ProjectileComponent_BP_C|GetHitTarget (Variables|Default|GetProjectileComponent_BP))
    (Actor|DestroyActor)))

(fn ConstructionScript)