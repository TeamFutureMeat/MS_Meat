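; Greedy boss actor with a power-on intro, face states driven by UV animation and material parameters, and health-based attacks against the player.
; The attack routine summons when its enemy count is zero, otherwise picking throw, random two-attack combos or rabbit by HP, scheduled with named timers.
; Timelines drive body bobbing and arm morphs, feeding snack-bag missile and coin-spawning moves.
; Several attacks only set damage, counters or debug prints.
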(event Custom|Arm%20Opening%20And%20Closing
  (params (Open :type Boolean) (Default :type Boolean))
  (bind _mesh (Variables|Character|GetMesh))
  ;[1 1 1] アームの開閉
  (if Default
    (Components|SkeletalMesh|SetMorphTarget _mesh "Open" 0.0 false)
    (Components|SkeletalMesh|SetMorphTarget _mesh "Close" 0.0 false)
    (elif Open
      (bind (_direction _open_morph_weight _colse_morph_weight) (Timeline|Open PlayFromStart)
        (:Update
          (Components|SkeletalMesh|SetMorphTarget _mesh "Open" _open_morph_weight false)
          (Components|SkeletalMesh|SetMorphTarget _mesh "Close" _colse_morph_weight false)))
      (else
        (bind (_direction_2 _colse_morph_weight_2 _open_morph_weight_2) (Timeline|Colse PlayFromStart)
          (:Update
            (Components|SkeletalMesh|SetMorphTarget _mesh "Open" _open_morph_weight_2 false)
            (Components|SkeletalMesh|SetMorphTarget _mesh "Close" _colse_morph_weight_2 false)))))))

(event Custom|SnackMissileSet_Event
  (bind _mesh (Variables|Character|GetMesh))
  (bind _returnvalue (Transformation|GetWorldLocation _mesh))
  ;[1 1 1] お菓子ミサイルムーブ
  (bind _上下移動 (Timeline|タイムライン_0 PlayFromStart)
    (:Update
      (Transformation|SetWorldLocation (Variables|Character|GetMesh) (Math|Vector|MakeVector (.x _returnvalue) (.y _returnvalue) (+ (.z (Variables|Default|GetInitialLocation)) _上下移動)) false false))
    (:Finished
      (Default|SetIsFireMissile (Variables|Default|GetSnackBag) true))
    (:SpawnEvent
      (CallFunction|SpawnSnackBag)
      (CallFunction|ArmOpeningandClosing false false)
      (Default|PlayAnimation (Variables|Default|GetAnimBP) "NewEnumerator1"))))

(event Custom|Power%20On
  ;[1 1 1] 登場時の起動演出ムーブ
  (bind (_direction _sub_texture_blend _face_color) (Timeline|Power%20On%20TimeLine Play)
    (:Update
      (Rendering|Material|SetScalarParameterValueonMaterials (Variables|Character|GetMesh) "SubTextureBlend" _sub_texture_blend)
      (CallFunction|ChangeFaceColor false _face_color)
      (Default|SetAutoChageAniamationFlag (Variables|Default|GetUV_Animation_BP) false))
    (:Finished
      (Default|SetAutoChageAniamationFlag (Variables|Default|GetUV_Animation_BP) true)
      (CallFunction|IdleState)
      (Utilities|FlowControl|Delay 2.0)
      (CallFunction|WelcomeState))))

(event Custom|SnackMissile%20Update_Event
  ;[1 1 1] お菓子ミサイルムーブ
  (bind _flag (Default|GetIsEmpty (Variables|Default|GetSnackBag)))
  (if _flag
    (CallFunction|ArmOpeningandClosing false true)
    (Default|PlayAnimation (Variables|Default|GetAnimBP) "NewEnumerator6")))

(event Custom|Call%20The%20Coins%20Event
  (bind _mesh (Variables|Character|GetMesh))
  (bind _returnvalue (Transformation|GetWorldLocation _mesh))
  (CallFunction|SpawntheCoins)
  (bind _上下移動 (Timeline|Call%20The%20Coin PlayFromStart)
    (:Update
      (Transformation|SetWorldLocation _mesh (Math|Vector|MakeVector (.x _returnvalue) (.y _returnvalue) (+ (.z (Variables|Default|GetInitialLocation)) _上下移動)) false false))))

(event EventBeginPlay
  (Default|UVAnimationInitialize (Variables|Default|GetUV_Animation_BP) (Variables|Character|GetMesh) "Greedy_face_inside_MT")
  (CallFunction|InitializeAnimation)
  (Variables|Default|SetNowHitPoint (Variables|Default|GetMaxHitPoint))
  (bind _asplayer (Utilities|Casting|CastToPlayer (Game|Player|GetPlayerPawn 0)))
  (Variables|Default|SetTarget _asplayer)
  (Variables|Default|SetInitialLocation (Transformation|GetWorldLocation (Variables|Character|GetMesh))))

(event Collision|EventActorBeginOverlap
  (params (OtherActor :type Actor%20Object%20Reference)))

(event EventTick
  (params (DeltaSeconds :type Float%20%28single-precision%29))
  (Utilities|FlowControl|Sequence
    (:then_0
      (bind _now_animation (Default|GetNowAnimation (Variables|Default|GetAnimBP)))
      (switch Utilities|FlowControl|Switch|SwitchonGreedy_AnimationPattern _now_animation
        (:NewEnumerator1
          (CallFunction|SnackMissileUpdateEvent))))
    (:then_1
      (if (!= (Variables|Default|GetNowFacePattern) (Variables|Default|GetOldFacePattern))
        (Variables|Default|SetOldFacePattern (Variables|Default|GetNowFacePattern))))))

(fn ConstructionScript)

(fn IdleState
  (Default|PlayAnimation (Variables|Default|GetAnimBP) "NewEnumerator0")
  (CallFunction|SetNowFacePattern "NewEnumerator0")
  (CallFunction|ChangeFaceColor false "0,0.500000,1.000000"))

(fn WelcomeState
  (CallFunction|SetNowFacePattern "NewEnumerator10")
  (CallFunction|ChangeFaceColor true "1.000000,1.000000,1.000000"))

(fn StopState
  (Default|PlayAnimation (Variables|Default|GetAnimBP) "NewEnumerator7")
  (CallFunction|ChangeFaceColor false "0, 0, 0"))

(fn SmileState
  (CallFunction|SetNowFacePattern "NewEnumerator12")
  (CallFunction|ChangeFaceColor false "1.000000,1.000000,0.000000"))

(fn ChangeFaceColor
  (params (Rainbow :type Boolean) (Color :type Vector))
  (bind _mesh (Variables|Character|GetMesh))
  (if Rainbow
    (Rendering|Material|SetScalarParameterValueonMaterials _mesh "RainbowBlend" 1.0)
    (else
      (Rendering|Material|SetScalarParameterValueonMaterials _mesh "RainbowBlend" 0.0)))
  (Rendering|Material|SetVectorParameterValueonMaterials _mesh "EmissiveColor" Color))

(fn GreedyAttackPaternNAGE
  (Variables|Default|SetDamage (* (Variables|Default|GetAttackDamage) 1.0))
  (if (> (Variables|Default|GetNowHaveEnemyNum) 0)
    (bind _output_get (Variables|Default|SetNowHaveEnemyNum (- (Variables|Default|GetNowHaveEnemyNum) 1)))
    (Development|PrintString "グリーディー-敵投げ")
    (Development|PrintString (Utilities|String|ToString(Integer) _output_get))))

(fn GreedyAttackPaternSYOUSYU
  (Variables|Default|SetNowHaveEnemyNum 5))

(fn GreedyAttackPaternMISSILE
  (Variables|Default|SetDamage (* (Variables|Default|GetAttackDamage) 1.2))
  (CallFunction|SnackMissileSetEvent))

(fn GreedyAttackPaternRABBIT
  (Variables|Default|SetDamage (* (Variables|Default|GetAttackDamage) 2.0)))

(fn GreedyRoutine
  (bind _output_get (Variables|Default|Setrand (Math|Random|RandomInteger 4)))
  (Development|PrintString (Utilities|String|ToString(Integer) _output_get))
  (switch int _output_get
    (:0
      (Utilities|Time|SetTimerbyFunctionName 0 "Greedy_AttackPatern_NAGE" (Variables|Default|GetAttackWaitTime))
      (bind _returnvalue (Utilities|Time|SetTimerbyFunctionName 0 "Greedy_AttackPatern_MISSILE" (* (+ (Variables|Default|GetAttackWaitTime) 0.0) 2.0))))
    (:1
      (Utilities|Time|SetTimerbyFunctionName 0 "Greedy_AttackPatern_NAGE" (Variables|Default|GetAttackWaitTime))
      (bind _returnvalue_2 (Utilities|Time|SetTimerbyFunctionName 0 "Greedy_AttackPatern_NAGE" (* (+ (Variables|Default|GetAttackWaitTime) 0.0) 2.0))))
    (:2
      (Utilities|Time|SetTimerbyFunctionName 0 "Greedy_AttackPatern_RABBIT" (Variables|Default|GetAttackWaitTime))
      (bind _returnvalue_3 (Utilities|Time|SetTimerbyFunctionName 0 "Greedy_AttackPatern_RABBIT" (* (+ (Variables|Default|GetAttackWaitTime) 0.0) 2.0))))
    (:3
      (Utilities|Time|SetTimerbyFunctionName 0 "Greedy_AttackPatern_RABBIT" (Variables|Default|GetAttackWaitTime))
      (bind _returnvalue_4 (Utilities|Time|SetTimerbyFunctionName 0 "Greedy_AttackPatern_NAGE" (* (+ (Variables|Default|GetAttackWaitTime) 0.0) 2.0)))))
  (return (Utilities|Array|MakeArray _returnvalue _returnvalue_2 _returnvalue_3 _returnvalue_4)))

(fn SpawnSnackBag
  (bind _returnvalue (Game|SpawnActorfromClass "/Game/Throbrave/Model/Greedy/BP/SnackBag_BP.SnackBag_BP_C" (Transformation|GetSocketTransform (Variables|Character|GetMesh) "SnackBagSocket" "RTS_World") "Undefined" 0 (Variables|Default|GetTarget) self 0))
  (Variables|Default|SetSnackBag _returnvalue))

(fn SetNowFacePattern
  (params (Face%20Pattern :type Greedy_FaceAnimationPattern%20Enum :default "NewEnumerator0"))
  (if (!= (Variables|Default|GetNowFacePattern) Face%20Pattern)
    (bind _output_get (Variables|Default|SetNowFacePattern Face%20Pattern))
    (Default|SetNowState (Variables|Default|GetUV_Animation_BP) (.Value (Utilities|Map|Find (Variables|Default|GetFaceAnimationPattern) _output_get)))))

(fn InitializeAnimation
  (bind _asgreedy_anim_bp (Utilities|Casting|CastToGreedy_AnimBP (Components|SkeletalMesh|GetAnimInstance (Variables|Character|GetMesh))))
  (bind _output_get (Variables|Default|SetAnimBP _asgreedy_anim_bp))
  (Default|SetGreedyBP _output_get self)
  (Rendering|Material|SetScalarParameterValueonMaterials (Variables|Character|GetMesh) "SubTextureBlend" 0.0)
  (CallFunction|IdleState))

(fn SpawntheCoins
  (bind _box (Variables|Default|GetBox))
  (for _index (range 0 (Variables|Default|GetThe%20Coin%20Max%20SpawnNum))
    (bind _returnvalue (Game|SpawnActorfromClass "/Game/Throbrave/Model/TheCoin/BP/The_Coin.The_Coin_C" (Math|Transform|MakeTransform (Math|Random|RandomPointinBoundingBox (.location (Transformation|GetRelativeTransform _box)) (Components|Box|GetScaledBoxExtent _box)) "0, 0, 0" "1,1,1") "Undefined" 0 0))
    (Utilities|Array|Add (Variables|Default|GetThe%20Coins) _returnvalue)
    (Default|SetIsCanMove _returnvalue false)))