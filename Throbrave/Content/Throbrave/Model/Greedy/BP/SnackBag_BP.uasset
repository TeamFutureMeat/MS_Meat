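; SnackBag_BP is a snack bag actor that spawns a limited number of OkasiMissile_BP actors, passing each a MissileTarget.
; On Tick it spawns the next missile at the bag's socket whenever the previous one is no longer valid.
; Each spawn raises a target morph weight, which the bag's morph target approaches in small per-tick steps.
; Once the count runs out and the last missile is gone, the bag enables gravity.
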(event EventBeginPlay)

(event Collision|EventActorBeginOverlap
  (params (OtherActor :type Actor%20Object%20Reference)))

(event EventTick
  (params (DeltaSeconds :type Float%20%28single-precision%29))
  (if (Variables|Default|GetIsEmpty)
    (Physics|SetEnableGravity (Variables|Default|GetBag) true)
    (else
      (CallFunction|UpdateSnackMissile)
      (CallFunction|UpdateMorphing))))

(fn ConstructionScript)

(fn UpdateSnackMissile
  (if (not (Utilities|IsValid (Variables|Default|GetNowMissile)))
    (if (<= (Variables|Default|GetSnackMissileNum) (Variables|Default|GetNowMissileNum))
      (Variables|Default|SetIsEmpty true)
      (else
        (CallFunction|SpawnSnackMissile)
        (CallFunction|SetMorphWeight)))))

(fn SpawnSnackMissile
  (bind _returnvalue (Game|SpawnActorfromClass "/Game/Throbrave/Model/Greedy/BP/OkasiMissile_BP.OkasiMissile_BP_C" (Math|Transform|MakeTransform (.location (Transformation|GetSocketTransform (Variables|Default|GetBag) "SnackMissile_Socket" "RTS_World")) "-220.000000, 0, 0" "5.000000,5.000000,5.000000") "Undefined" 0 (Variables|Default|GetMissileTarget) 0))
  (Variables|Default|SetNowMissile _returnvalue)
  (bind _result (Math|Integer|IncrementInt (Variables|Default|GetNowMissileNum))
    (:%20%20
      (Variables|Default|SetNowMissileNum _result))))

(fn SetMorphWeight
  (Variables|Default|SetMorphWeight (* (/ 1.0 (Math|Conversions|ToFloat(Integer) (Variables|Default|GetSnackMissileNum))) (Math|Conversions|ToFloat(Integer) (Variables|Default|GetNowMissileNum)))))

(fn UpdateMorphing
  (if (< (Variables|Default|GetNowMorph%20Weight) (Variables|Default|GetMorphWeight))
    (Variables|Default|SetNowMorph%20Weight (+ (Variables|Default|GetNowMorph%20Weight) 0.01))
    (Components|SkeletalMesh|SetMorphTarget (Variables|Default|GetBag) "Snack_bag_model1" (Math|Float|Lerp 0.0 1.0 (Variables|Default|GetNowMorph%20Weight)) false)))