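; UV animation Blueprint that animates a skeletal mesh material by shifting texture coordinates per animation state.
; Initialization creates a dynamic material instance on a named slot, driven through Width and Height scalar parameters.
; Tick optionally advances to each pattern's next state after its interval, then applies the current state's UV position from a data map.
; Scrolling patterns move along their vector until a one-unit limit, resetting if looped.
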(event EventBeginPlay)

(event EventTick
  (params (DeltaSeconds :type Float%20%28single-precision%29))
  (Variables|Default|SetNowGameTime (Utilities|Time|GetGameTimeinSeconds))
  (CallFunction|AutoChangeAnimationPattern)
  (CallFunction|ChangeAnimationPattern)
  (CallFunction|ScrollAnimationPattern))

(fn CreateMaterialInstance(SkeletalMesh)
  (params (Mesh :type Skeletal%20Mesh%20Component%20Object%20Reference) (MaterialSlotName :type Name))
  (bind _returnvalue (Rendering|Material|GetMaterialIndex Mesh MaterialSlotName))
  (bind _returnvalue_2 (Rendering|Material|CreateDynamicMaterialInstance Mesh _returnvalue (Rendering|Material|GetMaterial Mesh _returnvalue) "None" :!class /Script/Engine.PrimitiveComponent))
  (Variables|Default|SetAnimation_Mesh _returnvalue_2))

(fn UVAnimationInitialize
  (params (Skeletal%20Mesh :type Skeletal%20Mesh%20Component%20Object%20Reference) (Material%20Slot%20Name :type Name))
  (デフォルト|CreateMaterialInstance(SkeletalMesh) Skeletal%20Mesh Material%20Slot%20Name))

(fn WidthScroll
  (params (Scroll%20Velue :type Float%20%28single-precision%29))
  (Rendering|Material|SetScalarParameterValue (Variables|Default|GetAnimation_Mesh) (Variables|Default|GetWidth) Scroll%20Velue :!class /Script/Engine.MaterialInstanceDynamic))

(fn HeightScroll
  (params (Scroll%20Value :type Float%20%28single-precision%29))
  (bind _animation_mesh (Variables|Default|GetAnimation_Mesh))
  (Rendering|Material|SetScalarParameterValue _animation_mesh (Variables|Default|GetHeight) Scroll%20Value :!class /Script/Engine.MaterialInstanceDynamic)
  (Rendering|Material|GetScalarParameterValue _animation_mesh "Height_Divid" :!class /Script/Engine.MaterialInstanceDynamic))

(fn ChangeAnimationPattern
  (bind _now_animation_state (Variables|Default|GetNow_Animation_State))
  (bind _animation_pattern_data (Variables|Default|GetAnimation_Pattern_Data))
  (bind _value (Utilities|Map|Find _animation_pattern_data _now_animation_state))
  (bind _uv_position (Utilities|Struct|BreakUV_Animation _value))
  (bind (_x _y) (Math|Vector2D|BreakVector2D _uv_position))
  (if (!= _now_animation_state (Variables|Default|GetOld%20_Animation_State))
    (CallFunction|WidthScroll _x)
    (CallFunction|HeightScroll _y)
    (Variables|Default|SetOld%20_Animation_State (Variables|Default|GetNow_Animation_State))
    (Variables|Default|SetU_Pos _x)
    (Variables|Default|SetV_Pos _y)))

(fn ScrollAnimationPattern
  (bind _animation_pattern_data (Variables|Default|GetAnimation_Pattern_Data))
  (bind _now_animation_state (Variables|Default|GetNow_Animation_State))
  (bind _value (Utilities|Map|Find _animation_pattern_data _now_animation_state))
  (bind (_scroll _scroll_looping _scroll_speed _scroll_vector _uv_position) (Utilities|Struct|BreakUV_Animation _value))
  (if _scroll
    (if (and (< (Variables|Default|GetU_Pos) (+ (.x _uv_position) 1.0)) (< (Variables|Default|GetV_Pos) (+ (.y _uv_position) 1.0)))
      (Variables|Default|SetU_Pos (+ (Variables|Default|GetU_Pos) (* _scroll_speed (.x _scroll_vector))))
      (Variables|Default|SetV_Pos (+ (Variables|Default|GetV_Pos) (* _scroll_speed (.y _scroll_vector))))
      (CallFunction|WidthScroll (Variables|Default|GetU_Pos))
      (CallFunction|HeightScroll (Variables|Default|GetV_Pos) :!label _label)
      (elif _scroll_looping
        (Variables|Default|SetU_Pos (.x _uv_position))
        (Variables|Default|SetV_Pos (.y _uv_position))
        (goto _label)))))

(fn AutoChangeAnimationPattern
  (bind _animation_pattern_data (Variables|Default|GetAnimation_Pattern_Data))
  (bind _now_animation_state (Variables|Default|GetNow_Animation_State))
  (bind _value (Utilities|Map|Find _animation_pattern_data _now_animation_state))
  (if (Variables|Default|GetAutoChage%20Flag)
    (if (!= (Utilities|Enum|LiteralenumEUV_Animation_State "NewEnumerator3") (.next_state _value))
      (if (>= (- (Variables|Default|GetNowGameTime) (Variables|Default|GetOldGameTime)) (.next_state_change_interval _value))
        (Development|PrintString (Utilities|String|ToString(Float) (.next_state_change_interval _value)))
        (CallFunction|SetNowState (.next_state _value))
        (Variables|Default|SetOldGameTime (Variables|Default|GetNowGameTime))))))

(fn SetNowState
  (params (State :type EUV_Animation_State%20Enum :default "NewEnumerator3"))
  (if (!= State (Variables|Default|GetNow_Animation_State))
    (Variables|Default|SetNow_Animation_State State)))

(fn UVAnimationFinalize
  (Utilities|Time|ClearTimerbyFunctionName 0 "AutoChangeAnimationPattern"))

(fn SetAutoChageAniamationFlag
  (params (flag :type Boolean))
  (Variables|Default|SetAutoChage%20Flag flag))