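; Enemy Blueprint that drives a periodic attack through an EnemyAttack widget.
; On BeginPlay it creates the EnemyAttack widget, stores it and adds it to the viewport.
; Tick increments a frame-based counter and, once it passes a fixed threshold, calls Attack on the widget and resets it, so attack timing depends on frame rate.
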(event EventBeginPlay
  (bind _returnvalue (UserInterface|CreateWidget "/Game/CR_HERO/Widget/EnemyAttack.EnemyAttack_C"))
  (bind _output_get (Variables|Default|SetEnemyAttack _returnvalue))
  (UserInterface|Viewport|AddtoViewport _output_get 0))

(event Collision|EventActorBeginOverlap
  (params (OtherActor :type Actor%20Object%20Reference)))

(event EventTick
  (params (DeltaSeconds :type Float%20%28single-precision%29))
  (bind _result (Math|Float|IncrementFloat (Variables|Default|GetAttackCount))
    (:%20%20
      (bind _output_get (Variables|Default|SetAttackCount _result))
      (if (> _output_get 3e+02)
        (Default|Attack (Variables|Default|GetEnemyAttack))
        (Variables|Default|SetAttackCount 0.0)))))

(fn ConstructionScript)