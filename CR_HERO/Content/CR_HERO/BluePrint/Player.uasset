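; Player Blueprint that turns Left, Up and Right key presses into left, center, right or simultaneous push calls.
; Each key press branches on its SimultaneousPush check, calling either the shared simultaneous push or that key's own push.
; The SimultaneousPush graphs test whether both other keys are held, though those expressions appear unused in the graphs.
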(event EventBeginPlay)

(event Collision|EventActorBeginOverlap
  (params (OtherActor :type Actor%20Object%20Reference)))

(event EventTick
  (params (DeltaSeconds :type Float%20%28single-precision%29)))

(event Input|KeyboardEvents|Left
  (params (Key :type Key%20Structure :default "None"))
  (:Pressed
    (if (Utilities|SimultaneousPushL)
      (Default|CallPushSimultaneous)
      (else
        (Default|CallPushLeft)))))

(event Input|KeyboardEvents|Up
  (params (Key :type Key%20Structure :default "None"))
  (:Pressed
    (if (Utilities|SimultaneousPushC)
      (Default|CallPushSimultaneous)
      (else
        (Default|CallPushCenter)))))

(event Input|KeyboardEvents|Right
  (params (Key :type Key%20Structure :default "None"))
  (:Pressed
    (if (Utilities|SimultaneousPushR)
      (Default|CallPushSimultaneous)
      (else
        (Default|CallPushRight)))))

(fn ConstructionScript)