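; GuardBP_ is a guard trigger that forwards a key press to the guard logic in MyGameInstance.
; Pressing E sets a GuardStart flag and calls StartGuard on the game instance.
; While the flag is set, Tick calls the game instance's Guard every frame, then clears the flag once GuardUIScaling is no longer above zero.
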(event EventTick
  (params (DeltaSeconds :type Float%20%28single-precision%29))
  (if (Variables|Default|GetGuardStart)
    (bind _asmy_game_instance (Utilities|Casting|CastToMyGameInstance (Game|GetGameInstance)))
    (Default|Guard _asmy_game_instance)
    (if (not (> (Variables|/Game/CR_HERO/MyGameInstance.MyGameInstance_C|GetGuardUIScaling _asmy_game_instance) 0.0))
      (Variables|Default|SetGuardStart false))))

(event Input|KeyboardEvents|E
  (params (Key :type Key%20Structure :default "None"))
  (:Pressed
    (Variables|Default|SetGuardStart true)
    (bind _asmy_game_instance (Utilities|Casting|CastToMyGameInstance (Game|GetGameInstance)))
    (Default|StartGuard _asmy_game_instance)))

(fn ConstructionScript)